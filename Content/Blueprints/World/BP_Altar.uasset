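; BP_Altar is a world checkpoint that registers a spawn point and triggers linked actors when the player touches its Ewer component.
; The overlap activates Niagara effects and passes the spawn name and priority to the jam GameMode.
; It then activates each ActorInteraction target, playing a sound per target.
; The Checked guard uses equality rather than AND, so non-player overlaps retrigger it once checked.
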(event OnComponentBeginOverlap(ewer)
  (params (OverlappedComponent :type Primitive%20Component%20Object%20Reference) (OtherActor :type Actor%20Object%20Reference) (OtherComp :type Primitive%20Component%20Object%20Reference) (OtherBodyIndex :type Integer) (bFromSweep :type Boolean) (SweepResult :type Hit%20Result%20Structure%20%28by%20ref%29))
  (if (== (== OtherActor (Game|Player|GetPlayerPawn 0)) (not (Variables|Default|GetChecked)))
    (Variables|Default|SetChecked true)
    (Components|Activation|Activate (Variables|Default|GetNiagara) false)
    (bind _asgdtv_jam_2022game_mode_base (Utilities|Casting|CastToGDTV_Jam_2022GameModeBase (Game|GetGameMode)))
    (Class|GDTVJam2022GameModeBase|ActivateSpawnPoint _asgdtv_jam_2022game_mode_base (Variables|Default|GetSpawnName) (Variables|Default|GetSpawnPrio))
    (for _array_element (Variables|Default|GetTarget)
      (bind _asactor_interaction (Utilities|Casting|CastToActorInteraction _array_element))
      (Default|Activate _asactor_interaction)
      (Audio|PlaySoundatLocation (Variables|Default|GetSound) (Transformation|GetActorLocation) "0, 0, 0" 1.0 1.0 0.0 0 0 0 0))))

(event EventBeginPlay)

(event Collision|EventActorBeginOverlap
  (params (OtherActor :type Actor%20Object%20Reference)))

(event EventTick
  (params (DeltaSeconds :type Float%20%28single-precision%29)))

(fn ConstructionScript)