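; SequenceManager is a world Blueprint that lets the player cancel a running sequence with Escape.
; The key press stops and clears SequencePlayer, hands input back from itself to the player pawn, and removes SequenceWidget.
; It also turns off the stored StartEnemy's IsPeacefull flag and clears that reference.
; Nothing here starts a sequence or assigns these references, and ClearSequence is an empty stub.
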(event EventBeginPlay)

(event Collision|EventActorBeginOverlap
  (params (OtherActor :type Actor%20Object%20Reference)))

(event EventTick
  (params (DeltaSeconds :type Float%20%28single-precision%29)))

(event Input|ActionEvents|InputActionEscape
  (params (Key :type Key%20Structure :default "None"))
  (bind _returnvalue (Game|GetPlayerController 0))
  (:Pressed
    (Utilities|FlowControl|Sequence
      (:then_0
        (Utilities|IsValid (Variables|Default|GetSequencePlayer)
          (:Is%20Valid
            (Sequencer|Player|Stop (Variables|Default|GetSequencePlayer) :!class /Script/MovieScene.MovieSceneSequencePlayer)
            (Variables|Default|SetSequencePlayer 0))))
      (:then_1
        (Input|DisableInput _returnvalue)
        (Input|EnableInput (Game|Player|GetPlayerPawn 0) _returnvalue))
      (:then_2
        (bind _sequencewidget (Variables|Default|GetSequenceWidget)
          (:then
            (Widget|RemovefromParent _sequencewidget)
            (Variables|Default|SetSequenceWidget 0))
          (:else)))
      (:then_3
        (bind _startenemy (Variables|Default|GetStartEnemy)
          (:then
            (Variables|/Script/GDTV_Jam_2022.Ghost|SetIsPeacefull _startenemy 0)
            (Variables|Default|SetStartEnemy 0))
          (:else))))))

(fn ConstructionScript)

(fn ClearSequence)