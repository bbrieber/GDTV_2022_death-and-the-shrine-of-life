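; Final altar actor that unlocks after enough Activate calls and triggers the end-game sequence when the player reaches it.
; On reaching the required count, it starts its activation Niagara effect and level sequence once and enables the capsule's overlap trigger.
; The player's first overlap plays the end-game sequence and effect, and sets every BP_Enemy peaceful.
; Each sequence player started is handed to SequenceManager.
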(event OnComponentBeginOverlap(Capsule)
  (params (OverlappedComponent :type Primitive%20Component%20Object%20Reference) (OtherActor :type Actor%20Object%20Reference) (OtherComp :type Primitive%20Component%20Object%20Reference) (OtherBodyIndex :type Integer) (bFromSweep :type Boolean) (SweepResult :type Hit%20Result%20Structure%20%28by%20ref%29))
  (bind _endgame_niagara (Variables|Default|GetEndGame_Niagara))
  (bind _endgameplayer (Variables|Default|GetEndGamePlayer))
  (if (== OtherActor (Game|Player|GetPlayerPawn 0))
    (Utilities|FlowControl|DoOnce false
      (:Completed
        (Utilities|FlowControl|Sequence
          (:then_0
            (Utilities|IsValid _endgameplayer
              (:Is%20Valid
                (Sequencer|Player|Play _endgameplayer :!class /Script/MovieScene.MovieSceneSequencePlayer)
                (Utilities|IsValid _endgame_niagara
                  (:Is%20Valid
                    (Components|Activation|Activate _endgame_niagara false)
                    (bind _sequencemanager (Variables|Default|GetSequenceManager)
                      (:then
                        (Variables|/Game/Blueprints/World/SequenceManager.SequenceManager_C|SetSequencePlayer _sequencemanager _endgameplayer))
                      (:else)))))))
          (:then_1
            (bind _outactors (Actor|GetAllActorsOfClass "/Game/Blueprints/Enemies/BP_Enemy.BP_Enemy_C"))
            (for _array_element _outactors
              (Variables|/Script/GDTV_Jam_2022.Ghost|SetIsPeacefull _array_element 1))))))))

(event EventBeginPlay
  (bind _activated_niagara (Variables|Default|GetActivated_Niagara))
  (bind _endgame_niagara (Variables|Default|GetEndGame_Niagara))
  (Utilities|FlowControl|Sequence
    (:then_0
      (bind _returnvalue (Sequencer|Player|CreateLevelSequencePlayer (Variables|Default|GetActivationSequence)))
      (Variables|Default|SetActivatePlayer _returnvalue))
    (:then_1
      (bind _returnvalue_2 (Sequencer|Player|CreateLevelSequencePlayer (Variables|Default|GetEndGameSequence)))
      (Variables|Default|SetEndGamePlayer _returnvalue_2))
    (:then_2
      (Collision|SetCollisionEnabled (Variables|Default|GetCapsule) "NoCollision"))
    (:then_3
      (Utilities|IsValid _activated_niagara
        (:Is%20Valid
          (Components|Activation|Deactivate _activated_niagara)
          (Utilities|IsValid _endgame_niagara
            (:Is%20Valid
              (Components|Activation|Deactivate _endgame_niagara))))))))

(event EventActivate
  (bind _activated_niagara (Variables|Default|GetActivated_Niagara))
  (bind _activateplayer (Variables|Default|GetActivatePlayer))
  (bind _result (Math|Integer|IncrementInt (Variables|Default|GetActivationCount))
    (:%20%20
      (if (>= _result (Variables|Default|GetNumToActivate))
        (Variables|Default|SetIsActive true)
        (Utilities|FlowControl|DoOnce false
          (:Completed
            (Utilities|IsValid _activated_niagara
              (:Is%20Valid
                (Components|Activation|Activate _activated_niagara false))
              (:Is%20Not%20Valid
                _))
            (Collision|SetCollisionEnabled (Variables|Default|GetCapsule) "QueryOnly")
            (Utilities|IsValid _activateplayer
              (:Is%20Valid
                (Sequencer|Player|Play _activateplayer :!class /Script/MovieScene.MovieSceneSequencePlayer)
                (bind _sequencemanager (Variables|Default|GetSequenceManager)
                  (:then
                    (Variables|/Game/Blueprints/World/SequenceManager.SequenceManager_C|SetSequencePlayer _sequencemanager (Variables|Default|GetActivatePlayer)))
                  (:else))))))))))

(fn ConstructionScript)