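; Player Blueprint for the Death game, with a Niagara wheel dust effect and an otherwise empty event graph.
; AdjustDustAmount stops dust spawning while the movement component is falling and restores a low spawn rate otherwise, but its only call is disconnected.
; Tick and Restarted are empty, and the DeathPlayerController HUD add and remove calls are unwired leftovers that never run.
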(event EventBeginPlay)

(event Collision|EventActorBeginOverlap
  (params (OtherActor :type Actor%20Object%20Reference)))

(event EventTick
  (params (DeltaSeconds :type Float%20%28single-precision%29)))

(event EventRestarted)

(fn ConstructionScript)

(fn AdjustDustAmount
  (bind _ns_wheeldust (Variables|Default|GetNS_WheelDust))
  (if (AI|Components|NavMovement|IsFalling (Pawn|GetMovementComponent))
    (Niagara|SetNiagaraVariable(Float) _ns_wheeldust "SpawnRate" 0.0)
    (else
      (Niagara|SetNiagaraVariable(Float) _ns_wheeldust "SpawnRate" 5.0))))

(fn NewFunction0)