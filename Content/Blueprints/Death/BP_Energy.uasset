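; BP_Energy is a health pickup that homes in on the player.
; Overlapping its DistanceTrigger with player pawn 0 starts a straight-line, unswept move toward the player each Tick at Speed.
; A squared-distance check on Tick, rather than the empty Collider overlap, triggers collection.
; DestroyAndAddHealth spawns a Niagara spark, adds HealthAmount to the player's HealthComponent and destroys the actor.
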(event OnComponentBeginOverlap(Collider)
  (params (OverlappedComponent :type Primitive%20Component%20Object%20Reference) (OtherActor :type Actor%20Object%20Reference) (OtherComp :type Primitive%20Component%20Object%20Reference) (OtherBodyIndex :type Integer) (bFromSweep :type Boolean) (SweepResult :type Hit%20Result%20Structure%20%28by%20ref%29)))

(event OnComponentBeginOverlap(DistanceTrigger)
  (params (OverlappedComponent :type Primitive%20Component%20Object%20Reference) (OtherActor :type Actor%20Object%20Reference) (OtherComp :type Primitive%20Component%20Object%20Reference) (OtherBodyIndex :type Integer) (bFromSweep :type Boolean) (SweepResult :type Hit%20Result%20Structure%20%28by%20ref%29))
  (if (== (Variables|Default|GetPlayer) OtherActor)
    (Variables|Default|SetMoveTowardsPlayer true)))

(event EventBeginPlay
  (Variables|Default|SetPlayer (Game|Player|GetPlayerPawn 0)))

(event Collision|EventActorBeginOverlap
  (params (OtherActor :type Actor%20Object%20Reference)))

(event EventTick
  (params (DeltaSeconds :type Float%20%28single-precision%29))
  (bind _returnvalue (Transformation|GetActorLocation))
  (bind _player (Variables|Default|GetPlayer))
  (bind _returnvalue_2 (Transformation|GetActorLocation _player))
  (bind _returnvalue_3 (- _returnvalue_2 _returnvalue))
  (if (Variables|Default|GetMoveTowardsPlayer)
    (Utilities|FlowControl|Sequence
      (:then_0
        (if (< (Math|Vector|VectorLengthSquared _returnvalue_3) 2e+01)
          (CallFunction|DestroyandAddHealth)))
      (:then_1
        (Transformation|SetActorLocation (+ _returnvalue (* (* (Math|Vector|Normalize _returnvalue_3) DeltaSeconds) (Variables|Default|GetSpeed))) false false)))))

(fn ConstructionScript)

(fn DestroyandAddHealth
  (bind _player (Variables|Default|GetPlayer))
  (Niagara|SpawnSystematLocation "/Game/VFX/NS_EnergySparkImpact.NS_EnergySparkImpact" (Transformation|GetActorLocation))
  (Utilities|IsValid _player
    (:Is%20Valid
      (Class|HealthComponent|AddHealth (Actor|GetComponentbyClass _player "/Script/GDTV_Jam_2022.HealthComponent") (Variables|Default|GetHealth%20Amount))
      (Actor|DestroyActor))))