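; Enemy Blueprint that drops actors, likely energy pickups, on death and plays a sound.
; OnDeath loops up to a random count between MinEnergy and MaxEnergy, spawning actors at random offsets around the enemy, with DestroyActor called inside the loop body.
; The Destroyed and OnGhostDied events share one path that plays a sound at the enemy's location.
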(event EventBeginPlay)

(event Collision|EventActorBeginOverlap
  (params (OtherActor :type Actor%20Object%20Reference)))

(event EventTick
  (params (DeltaSeconds :type Float%20%28single-precision%29)))

(event EventOnDeath
  (for _index (range 0 (Math|Random|RandomIntegerinRange (Variables|Default|GetMin%20Energy) (Variables|Default|GetMaxEnergy)))
    (Game|SpawnActorfromClass (Variables|Default|GetClass) (Math|Transform|MakeTransform (+ (Transformation|GetActorLocation) (Math|Vector|MakeVector (Math|Random|RandomFloatinRange -5e+01 5e+01) (Math|Random|RandomFloatinRange -5e+01 5e+01) (Math|Random|RandomFloatinRange -5e+01 5e+01)))) "Undefined" 0 0)
    (Actor|DestroyActor)))

(event EventDestroyed
  (Audio|PlaySoundatLocation (Variables|Default|GetSound) (Transformation|GetActorLocation) "0, 0, 0" 1.0 1.0 0.0 0 0 0 0))

(event EventOnGhostDied
  (Audio|PlaySoundatLocation (Variables|Default|GetSound) (Transformation|GetActorLocation) "0, 0, 0" 1.0 1.0 0.0 0 0 0 0))

(fn ConstructionScript)